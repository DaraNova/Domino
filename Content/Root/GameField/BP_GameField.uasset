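; BP_GameField is the game field actor that builds a rectangular grid of cells and its visible lines in the construction script.
; Two instanced static mesh components draw scaled, local-space lines from GridOrigin, with the horizontal set re-added for each vertical line by a nested loop.
; GridOrigin is then set to the actor location, and GridCells is refilled row by row with each cell's indices and corner position.
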(event EventBeginPlay)

(event Collision|EventActorBeginOverlap
  (params (OtherActor :type Actor%20Object%20Reference)))

(event EventTick
  (params (DeltaSeconds :type Float%20%28single-precision%29)))

(fn ConstructionScript
  (bind _cellsize_ (Variables|Default|GetCellSize%20))
  (bind _gridwidth_ (Variables|Default|GetGridWidth%20))
  (bind _cellsize__2 (Variables|Default|GetCellSize%20))
  (bind _gridheight_ (Variables|Default|GetGridHeight%20))
  (bind _returnvalue (* _gridheight_ _cellsize_))
  (bind _returnvalue_2 (* _gridwidth_ _cellsize__2))
  (Utilities|FlowControl|Sequence
    (:then_0
      (Components|InstancedStaticMesh|ClearInstances (Variables|Default|GetISM_VerticalLines))
      (Components|InstancedStaticMesh|ClearInstances (Variables|Default|GetISM_HorizontalLines))
      (for _index (range 0 (Variables|Default|GetGridWidth%20))
        (Components|InstancedStaticMesh|AddInstance (Variables|Default|GetISM_VerticalLines) (Math|Transform|MakeTransform (Math|Vector|MakeVector (+ (.x (Variables|Default|GetGridOrigin%20)) (* _index (Variables|Default|GetCellSize%20))) (+ (.y (Variables|Default|GetGridOrigin%20)) (/ _returnvalue 2.0)) (+ (.z (Variables|Default|GetGridOrigin%20)) 1.0)) "0, 0, 0" (Math|Vector|MakeVector 0.02 (/ _returnvalue 1e+02) 0.02)) false)
        (for _index_2 (range 0 (Variables|Default|GetGridHeight%20))
          (Components|InstancedStaticMesh|AddInstance (Variables|Default|GetISM_HorizontalLines) (Math|Transform|MakeTransform (Math|Vector|MakeVector (+ (.x (Variables|Default|GetGridOrigin%20)) (/ _returnvalue_2 2.0)) (+ (.y (Variables|Default|GetGridOrigin%20)) (* (Variables|Default|GetCellSize%20) _index_2)) (+ (.z (Variables|Default|GetGridOrigin%20)) 1.0)) "0, 0, 0" (Math|Vector|MakeVector (/ _returnvalue_2 1e+02) 0.02 0.02)) false))))
    (:then_1
      (Variables|Default|SetGridOrigin%20 (Transformation|GetActorLocation))
      (Utilities|Array|Clear (Variables|Default|GetGridCells%20))
      (for _index_3 (range 0 (- (Variables|Default|GetGridHeight%20) 1))
        (for _index_4 (range 0 (- (Variables|Default|GetGridWidth%20) 1))
          (Utilities|Array|Add (Variables|Default|GetGridCells%20) (Utilities|Struct|MakeST_GridCell _index_4 _index_3 false 0 (Math|Vector|MakeVector (+ (.x (Variables|Default|GetGridOrigin%20)) (* _index_4 (Variables|Default|GetCellSize%20))) (+ (.y (Variables|Default|GetGridOrigin%20)) (* _index_3 (Variables|Default|GetCellSize%20))) (.z (Variables|Default|GetGridOrigin%20))))))))))