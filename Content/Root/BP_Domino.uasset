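; BP_Domino is a clickable domino actor that can be selected and rotated until it is placed.
; Clicking its Cube does nothing once IsPlaced is set.
; Otherwise, the first click stores the domino as SelectedDomino and resets its yaw to zero.
; Further clicks while it remains selected turn it in quarter-turn steps around Z.
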(event OnClicked(Cube)
  (params (TouchedComponent :type Primitive%20Component%20Object%20Reference) (ButtonPressed :type Key%20Structure :default "None"))
  (bind _self self)
  (if (not (Variables|Default|GetbIsPlaced))
    (if (== (Variables|Default|GetSelectedDomino) _self)
      (bind _output_get (Variables|Default|SetCurrentRotation (+ (Variables|Default|GetCurrentRotation) 9e+01)))
      (Transformation|SetActorRotation (Math|Rotator|MakeRotator 0.0 0.0 _output_get))
      (else
        (Variables|Default|SetSelectedDomino _self)
        (bind _output_get_2 (Variables|Default|SetCurrentRotation 0.0))
        (Transformation|SetActorRotation (Math|Rotator|MakeRotator 0.0 0.0 _output_get_2))))))

(fn ConstructionScript)