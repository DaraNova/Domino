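; BP_RecipeBookmarkExtremeEasy is a clickable bookmark actor for one active recipe slot on the player's GameField.
; Clicking the Bookmark component asks the GameField to try completing the slot at RecipeSlotIndex.
; Hovering creates a new WBP_RecipeTooltip from that slot's recipe data and adds it to the viewport.
; Ending the hover only collapses the tooltip, leaving it in the viewport.
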(event OnClicked(bookmark)
  (params (TouchedComponent :type Primitive%20Component%20Object%20Reference) (ButtonPressed :type Key%20Structure :default "None"))
  (bind _asbp_player (Utilities|Casting|CastToBP_Player (Game|Player|GetPlayerPawn 0)))
  (Default|TryCompleteRecipeSlot (Variables|/Game/Root/BP_Player.BP_Player_C|GetGameField _asbp_player) (Variables|Default|GetRecipeSlotIndex)))

(event OnBeginCursorOver(bookmark)
  (params (TouchedComponent :type Primitive%20Component%20Object%20Reference))
  (bind _asbp_player (Utilities|Casting|CastToBP_Player (Game|Player|GetPlayerPawn 0)))
  (bind _returnvalue (UserInterface|CreateWidget "/Game/Root/UI/WBP_RecipeTooltip.WBP_RecipeTooltip_C" 0 (Utilities|Array|Get(acopy) (Variables|/Game/Root/GameField/BP_GameField.BP_GameField_C|GetActiveRecipeSlots (Variables|/Game/Root/BP_Player.BP_Player_C|GetGameField _asbp_player)) (Variables|Default|GetRecipeSlotIndex))))
  (bind _output_get (Variables|Default|SetTooltipRef _returnvalue))
  (UserInterface|Viewport|AddtoViewport _output_get 0))

(event OnEndCursorOver(bookmark)
  (params (TouchedComponent :type Primitive%20Component%20Object%20Reference))
  (Widget|SetVisibility (Variables|Default|GetTooltipRef) "Collapsed"))

(event EventBeginPlay)

(event Collision|EventActorBeginOverlap
  (params (OtherActor :type Actor%20Object%20Reference)))

(event EventTick
  (params (DeltaSeconds :type Float%20%28single-precision%29)))

(fn ConstructionScript)